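; TrafficLightGroup coordinates a list of traffic lights so they take turns, starting with the first light green at Begin Play.
; Tick times the active light through green, yellow and red, skipping zero-length green or yellow phases, and hands over after its red time.
; A frozen light halts the cycle, turning unfrozen lights red one per tick.
; The resume index derives from the frozen light's ID modulo two, suggesting paired lights.
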(event `self.ReceiveBeginPlay`
  (bind _trafficlights (`self.TrafficLights`))
  ;[1 1 1] Begin Play
  (if (> (`KismetArrayLibrary.Array_Length` _trafficlights) 0)
    (`/Game/Environment/Industrial/Props/TrafficLights/Blueprints/TrafficLights.Event on Traffic Light State Change` (`|GetArrayItem` _trafficlights) "NewEnumerator2")))

(event `self.ReceiveTick`
  (params (DeltaSeconds :type "Float (single-precision)"))
  (bind _output (`|GetArrayItem` (`self.TrafficLights`) (`self.AfterBreakTLID`)))
  (bind _output_2 (`|GetArrayItem` (`self.TrafficLights`) (`self.AfterBreakTLID`)))
  (bind _output_3 (`|GetArrayItem` (`self.TrafficLights`) (`self.Selected Traffic Light`)))
  ;[1 1 1] Each Step
  (for _array_element (`self.TrafficLights`)
    (if (`/Game/Environment/Industrial/Props/TrafficLights/Blueprints/TrafficLights.Freeze` _array_element)
      (set `self.BreakGroup` true)
      (set `self.AfterBreakTLID` (mod (+ (`/Game/Environment/Industrial/Props/TrafficLights/Blueprints/TrafficLights.ID` _array_element) 1) 2))
      (set `/Game/Environment/Industrial/Props/TrafficLights/Blueprints/TrafficLights.TimeElapse` 0.0 _array_element)
      (break)
      (else
        (set `self.BreakGroup` false))))
  (if (`self.BreakGroup`)
    (if (not (`/Game/Environment/Industrial/Props/TrafficLights/Blueprints/TrafficLights.Freeze` _output_3))
      (`/Game/Environment/Industrial/Props/TrafficLights/Blueprints/TrafficLights.Event on Traffic Light State Change` _output_3 "NewEnumerator0"))
    (bind _result (`/Engine/EditorBlueprintResources/StandardMacros.IncrementInt` (`self.Selected Traffic Light`))
      (:`  `
        (if (== _result (`KismetArrayLibrary.Array_Length` (`self.TrafficLights`)))
          (set `self.Selected Traffic Light` 0)
          (set `/Game/Environment/Industrial/Props/TrafficLights/Blueprints/TrafficLights.TimeElapse` 0.0 _output_3))))
    (else
      (bind _output_get (set `/Game/Environment/Industrial/Props/TrafficLights/Blueprints/TrafficLights.TimeElapse` (+ (`/Game/Environment/Industrial/Props/TrafficLights/Blueprints/TrafficLights.TimeElapse` _output) DeltaSeconds) _output))
      (switch `/Game/Environment/Industrial/Props/TrafficLights/Enum-TrafficLightsState` (`/Game/Environment/Industrial/Props/TrafficLights/Blueprints/TrafficLights.CurrentState` _output)
        (:`NewEnumerator0`
          (if (<= (`/Game/Environment/Industrial/Props/TrafficLights/Blueprints/TrafficLights.RedTime` _output) _output_get)
            (bind _result_2 (`/Engine/EditorBlueprintResources/StandardMacros.IncrementInt` (`self.AfterBreakTLID`))
              (:`  `
                (if (== _result_2 (`KismetArrayLibrary.Array_Length` (`self.TrafficLights`)))
                  (set `self.AfterBreakTLID` 0))
                (set `/Game/Environment/Industrial/Props/TrafficLights/Blueprints/TrafficLights.TimeElapse` 0.0 _output_2 :!label _label)
                (switch `/Game/Environment/Industrial/Props/TrafficLights/Enum-TrafficLightsState` (`/Game/Environment/Industrial/Props/TrafficLights/Blueprints/TrafficLights.CurrentState` _output_2)
                  (:`NewEnumerator0`
                    (if (> (`/Game/Environment/Industrial/Props/TrafficLights/Blueprints/TrafficLights.GreenTime` _output_2) 0.0)
                      (`/Game/Environment/Industrial/Props/TrafficLights/Blueprints/TrafficLights.Event on Traffic Light State Change` _output_2 "NewEnumerator2")
                      (else
                        (if (> (`/Game/Environment/Industrial/Props/TrafficLights/Blueprints/TrafficLights.YellowTime` _output_2) 0.0) :!label _label_2
                          (`/Game/Environment/Industrial/Props/TrafficLights/Blueprints/TrafficLights.Event on Traffic Light State Change` _output_2 "NewEnumerator1")
                          (else
                            (`/Game/Environment/Industrial/Props/TrafficLights/Blueprints/TrafficLights.Event on Traffic Light State Change` _output_2 "NewEnumerator0" :!label _label_3))))))
                  (:`NewEnumerator1`
                    (goto _label_3))
                  (:`NewEnumerator2`
                    (goto _label_2)))))))
        (:`NewEnumerator1`
          (if (<= (`/Game/Environment/Industrial/Props/TrafficLights/Blueprints/TrafficLights.YellowTime` _output) _output_get)
            (goto _label)))
        (:`NewEnumerator2`
          (if (<= (`/Game/Environment/Industrial/Props/TrafficLights/Blueprints/TrafficLights.GreenTime` _output) _output_get)
            (goto _label)))))))

(fn `UserConstructionScript`)